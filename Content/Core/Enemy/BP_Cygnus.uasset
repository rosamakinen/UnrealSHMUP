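; BP_Cygnus is an enemy actor with placeholder attack and damage logic driven by debug keys.
; It enables player input on BeginPlay so K prints a message and spawns a BP_Projectile at a fixed world X offset from the actor.
; The debug Space Bar key calls TakeDamage, which subtracts a fixed amount from Health, printing the result or destroying the actor at zero or below.
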(event Custom|TakeDamage
  (Variables|Default|SetHealth (- (Variables|Default|GetHealth) 1e+01))
  (if (<= (Variables|Default|GetHealth) 0.0)
    (Development|PrintString "Enemy Died")
    (Actor|DestroyActor)
    (else
      (Development|PrintString "Boom")
      (Development|PrintString (Utilities|String|ToString(Float) (Variables|Default|GetHealth))))))

(event EventBeginPlay
  ;[1 1 1] Comment
  ;;[1 1 1] Needs to happen by itself, not from button press. DEBUG
  (Input|EnableInput (Game|GetPlayerController 0)))

(event Input|KeyboardEvents|DebugKeySpaceBar
  (params (Key :type Key%20Structure :default "None") (ActionValue :type Input%20Action%20Value%20Structure))
  (:Pressed
    (CallFunction|TakeDamage)))

(event Input|KeyboardEvents|K
  (params (Key :type Key%20Structure :default "None"))
  (bind _returnvalue (Transformation|GetActorTransform))
  ;[1 1 1] Comment
  (:Pressed
    (Development|PrintString "Hello")
    (Game|SpawnActorfromClass "/Game/Core/Assets/Projectile/BP_Projectile.BP_Projectile_C" (Math|Transform|MakeTransform (Math|Vector|MakeVector (+ (.x (.location _returnvalue)) 2e+02) (.y (.location _returnvalue)) (.z (.location _returnvalue))) "0, 0, 0" "1.000000,1.000000,1.000000") "Undefined" 0 0)))

(fn ConstructionScript)