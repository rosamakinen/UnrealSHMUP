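; Player character that adds an Enhanced Input mapping context and handles forward-axis movement, sideways dash and drill.
; Dash and drill use timelines to lerp actor location without sweep, along world Y by input and along +X respectively, each locked against re-triggering while running.
; Tick fires debug-drawn line traces both ways along Y from below the actor, setting left/right flags that block dashing; drill ignores them.
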(event Input|EnhancedActionEvents|EnhancedInputActionMyMove
  (params (ActionValue :type Vector%202D%20Structure) (ElapsedSeconds :type Float%20%28double-precision%29) (TriggeredSeconds :type Float%20%28double-precision%29) (InputAction :type Input%20Action%20Object%20Reference :default "/Game/Core/Input/Actions/MyMove.MyMove"))
  (:Triggered
    (Pawn|Input|AddMovementInput (Transformation|GetActorForwardVector) (.y ActionValue) false)
    (Variables|Default|SetDirection (Math|Vector2D|MakeVector2D 0.0 (.y ActionValue))))
  (:Started
    (Variables|Default|SetisHolding true))
  (:Completed
    (Variables|Default|SetisHolding false)))

(event Input|EnhancedActionEvents|EnhancedInputActionMyDash
  (params (ActionValue :type Vector%202D%20Structure) (ElapsedSeconds :type Float%20%28double-precision%29) (TriggeredSeconds :type Float%20%28double-precision%29) (InputAction :type Input%20Action%20Object%20Reference :default "/Game/Core/Input/Actions/MyDash.MyDash"))
  (:Started
    (Variables|Default|SetisPositive (> (.x ActionValue) 0.0))
    (if (not (Variables|Default|GetisDashing))
      (if (Variables|Default|GetisPositive)
        (if (not (Variables|Default|GetisBlockingRight))
          (Variables|Default|SetcurrentLocation (Transformation|GetActorLocation) :!label _label)
          (Variables|Default|SetendLocation (+ (Math|Vector|MakeVector 0.0 (* (.x ActionValue) 4e+02) 0.0) (Variables|Default|GetcurrentLocation)))
          (bind _alpha (Timeline|Timeline_0 PlayFromStart)
            (:Update
              (Variables|Default|SetisDashing true)
              (Development|PrintString (Utilities|String|ToString(Vector) (Math|Vector|Lerp(Vector) (Variables|Default|GetcurrentLocation) (Variables|Default|GetendLocation) _alpha)))
              (Transformation|SetActorLocation (Math|Vector|Lerp(Vector) (Variables|Default|GetcurrentLocation) (Variables|Default|GetendLocation) _alpha) false false))
            (:Finished
              (Variables|Default|SetisDashing false))))
        (elif (not (Variables|Default|GetisBlockingLeft))
          (goto _label))))))

(event Input|EnhancedActionEvents|EnhancedInputActionMyDrill
  (params (ActionValue :type Boolean) (ElapsedSeconds :type Float%20%28double-precision%29) (TriggeredSeconds :type Float%20%28double-precision%29) (InputAction :type Input%20Action%20Object%20Reference :default "/Game/Core/Input/Actions/MyDrill.MyDrill"))
  (:Triggered
    (if (not (Variables|Default|GetisDrilling))
      (Variables|Default|SetcurrentLocation (Transformation|GetActorLocation))
      (Variables|Default|SetendLocation (+ (Math|Vector|MakeVector 5e+03 0.0 0.0) (Variables|Default|GetcurrentLocation)))
      (bind _alpha (Timeline|Timeline_1 PlayFromStart)
        (:Update
          (Variables|Default|SetisDrilling true)
          (Development|PrintString (Utilities|String|ToString(Vector) (Math|Vector|Lerp(Vector) (Variables|Default|GetcurrentLocation) (Variables|Default|GetendLocation) _alpha)))
          (Transformation|SetActorLocation (Math|Vector|Lerp(Vector) (Variables|Default|GetcurrentLocation) (Variables|Default|GetendLocation) _alpha) false false))
        (:Finished
          (Variables|Default|SetisDrilling false))))))

(event EventTick
  (params (DeltaSeconds :type Float%20%28single-precision%29))
  (bind _returnvalue (Transformation|GetActorLocation))
  (bind _returnvalue_2 (- _returnvalue "0.000000,0.000000,250.000000"))
  (bind _returnvalue_3 (Collision|LineTraceByChannel _returnvalue_2 (+ _returnvalue_2 "0.000000,300.000000,0.000000") "TraceTypeQuery1" false 0 "ForOneFrame"))
  (bind _returnvalue_4 (Collision|LineTraceByChannel _returnvalue_2 (- _returnvalue_2 "0.000000,300.000000,0.000000") "TraceTypeQuery1" false 0 "ForOneFrame"))
  (Variables|Default|SetisBlockingRight _returnvalue_3)
  (Variables|Default|SetisBlockingLeft _returnvalue_4))

(event EventBeginPlay
  (bind _asplayer_controller (Utilities|Casting|CastToPlayerController (Pawn|GetController)))
  (Utilities|IsValid (PlayerController|LocalPlayerSubsystems|GetEnhancedInputLocalPlayerSubsystem _asplayer_controller)
    (:Is%20Valid
      (Input|AddMappingContext (PlayerController|LocalPlayerSubsystems|GetEnhancedInputLocalPlayerSubsystem _asplayer_controller) "/Game/Core/Input/IMC_MyInput.IMC_MyInput" 0 "(bIgnoreAllPressedKeysUntilRelease=True,bForceImmediately=False)"))))

(fn ConstructionScript)