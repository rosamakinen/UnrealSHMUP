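; BP_ScrollingField is a scrolling-level actor that spawns a single shape and slides it along the X axis.
; BeginPlay spawns a BP_Shape at the world origin, then runs the same Speed call that Tick repeats every frame.
; Speed moves the passed actor one unit in +X without sweep or delta-time scaling, so scroll rate depends on frame rate.
; Both BeginPlay and Speed print a debug "Hello".
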(event EventBeginPlay
  (bind _returnvalue (Game|SpawnActorfromClass "/Game/Core/ScrollingLevel/BP_Shape.BP_Shape_C" (Math|Transform|MakeTransform "0, 0, 0") "Undefined" 0 0))
  (Development|PrintString "Hello")
  (CallFunction|Speed _returnvalue))

(event Collision|EventActorBeginOverlap
  (params (OtherActor :type Actor%20Object%20Reference)))

(event EventTick
  (params (DeltaSeconds :type Float%20%28single-precision%29))
  (CallFunction|Speed (stale EventBeginPlay _returnvalue)))

(fn ConstructionScript)

(fn Speed
  (params (Actor :type Actor%20Object%20Reference))
  (bind _returnvalue (Transformation|GetActorLocation Actor))
  (Development|PrintString "Hello")
  (Transformation|SetActorLocation Actor (Math|Vector|MakeVector (+ (.x _returnvalue) 1.0) (.y _returnvalue) (.z _returnvalue)) false false))