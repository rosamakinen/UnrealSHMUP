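; BP_ScrollingField is a scrolling level Blueprint that moves eight referenced actors along negative X in an endless loop.
; Each Tick passes every actor to the Speed function, which steps it by a fixed, frame-rate-dependent offset.
; An actor reaching the rear limit jumps to a fixed far-forward position, which also resets its Y and Z.
; Calls for two more actors and a BP_Shape spawn are unconnected.
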(event EventBeginPlay)

(event Collision|EventActorBeginOverlap
  (params (OtherActor :type Actor%20Object%20Reference)))

(event EventTick
  (params (DeltaSeconds :type Float%20%28single-precision%29))
  (CallFunction|Speed (Variables|Components|GetActor2))
  (CallFunction|Speed (Variables|Components|GetAtcor))
  (CallFunction|Speed (Variables|Components|GetActor1))
  (CallFunction|Speed (Variables|Components|GetActor3))
  (CallFunction|Speed (Variables|Components|GetActor4))
  (CallFunction|Speed (Variables|Components|GetActor5))
  (CallFunction|Speed (Variables|Components|GetActor6))
  (CallFunction|Speed (Variables|Components|GetActor7)))

(fn ConstructionScript)

(fn Speed
  (params (Actor :type Actor%20Object%20Reference))
  (bind _returnvalue (Transformation|GetActorLocation Actor))
  (bind _returnvalue_2 (+ (.x _returnvalue) -3e+01))
  (if (<= _returnvalue_2 -1e+04)
    (Transformation|SetActorLocation Actor "90140.000000,0.000000,-140.500000" false false)
    (else
      (Transformation|SetActorLocation Actor (Math|Vector|MakeVector _returnvalue_2 (.y _returnvalue) (.z _returnvalue)) false false))))